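; Dialogue component that shows an NPC's lines in a WB_Dialogue widget, advancing one line per Interact call.
; The first call creates the widget with the speaker name and line; later calls update its text.
; Each data table row supplies the next row, table and end flag, forming a linked chain that can span tables.
; The call after an end-flagged line removes the widget, leaving the stored pointer for the next conversation.
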(event EventBeginPlay)

(event EventTick
  (params (DeltaSeconds :type Float%20%28single-precision%29)))

(event EventInteract
  (params (playerref :type BP%20Third%20Person%20Character%20Object%20Reference))
  (if (Variables|Default|GetEnddialogue)
    (Widget|RemovefromParent (Variables|Default|GetDialoguewidget))
    (Variables|Default|SetEnddialogue false)
    (Variables|Default|SetDialoguewidget 0)
    (else
      (Utilities|IsValid (Variables|Default|GetDialoguewidget)
        (:Is%20Valid
          (bind _returnvalue (Utilities|GetDataTableRow (Variables|Default|GetData%20Table) (Variables|Default|GetRow%20Name))
            (:then
              ;[0.15 0.15 0.15 0.5] Updates dialogue in order for NPC to say next line.
              (Default|UpdateDialogue (Variables|Default|GetDialoguewidget) (.Dialogue (Utilities|Struct|BreakDialogue_Structure _returnvalue)))
              (Variables|Default|SetRow%20Name (.Row (Utilities|Struct|BreakDialogue_Structure _returnvalue)))
              (Variables|Default|SetData%20Table (.Datatable (Utilities|Struct|BreakDialogue_Structure _returnvalue)))
              (Variables|Default|SetEnddialogue (.EndDialogue? (Utilities|Struct|BreakDialogue_Structure _returnvalue))))))
        (:Is%20Not%20Valid
          (bind _returnvalue_2 (Utilities|GetDataTableRow (Variables|Default|GetData%20Table) (Variables|Default|GetRow%20Name))
            (:then
              (bind _returnvalue_3 (UserInterface|CreateWidget "/Game/Dialogue/WB_Dialogue.WB_Dialogue_C" 0 (Utilities|Text|ToText(Name) (Variables|Default|GetName)) (.Dialogue (Utilities|Struct|BreakDialogue_Structure _returnvalue_2))))
              (bind _output_get (Variables|Default|SetDialoguewidget _returnvalue_3))
              (UserInterface|Viewport|AddtoViewport _output_get 0)
              (Variables|Default|SetRow%20Name (.Row (Utilities|Struct|BreakDialogue_Structure _returnvalue_2)))
              (Variables|Default|SetData%20Table (.Datatable (Utilities|Struct|BreakDialogue_Structure _returnvalue_2)))
              (Variables|Default|SetEnddialogue (.EndDialogue? (Utilities|Struct|BreakDialogue_Structure _returnvalue_2))))))))))